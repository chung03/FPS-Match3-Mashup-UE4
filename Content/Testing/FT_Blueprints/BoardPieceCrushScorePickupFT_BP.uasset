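; Functional test that checks a score pickup is destroyed when a board piece spawns on top of it.
; PrepareTest spawns a fast-spawning test board piece holder and a ScorePickUpBP just above it at the same horizontal position.
; StartTest waits briefly, asserts the pickup is no longer valid, finishes the test, then destroys the holder and any surviving pickup.
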(event `self.ReceivePrepareTest`
  (bind _returnvalue (`|SpawnActorFromClass` "/Game/Testing/ModifiedBPsForTest/Test_SpawnFastBoardPieceHolderType0BP.Test_SpawnFastBoardPieceHolderType0BP_C" (`KismetMathLibrary.MakeTransform` (0.0 500.0 0.0)) "Undefined" "OverrideRootScale" null null))
  (set `self.BoardPieceHolder1` _returnvalue)
  (bind _returnvalue_2 (`|SpawnActorFromClass` "/Game/FirstPersonCPP/Blueprints/ScorePickups/ScorePickUpBP.ScorePickUpBP_C" (`KismetMathLibrary.MakeTransform` (0.0 500.0 100.0)) "AlwaysSpawn" "OverrideRootScale" null null))
  (set `self.ScorePickUp1` _returnvalue_2))

(event `self.ReceiveStartTest`
  (bind _scorepickup1 (`self.ScorePickUp1`))
  (`KismetSystemLibrary.Delay` 1.0)
  (`self.AssertFalse` (`KismetSystemLibrary.IsValid` (`self.ScorePickUp1`)) "After Board Piece spawns on top of the Score Pick Up, the Score Pick Up should be destroyed")
  (`self.FinishTest` "Default")
  (`self.K2_DestroyActor` (`self.BoardPieceHolder1`))
  (`/Engine/EditorBlueprintResources/StandardMacros.IsValid` _scorepickup1
    (:`Is Valid`
      (`self.K2_DestroyActor` _scorepickup1))))

(fn `UserConstructionScript`)