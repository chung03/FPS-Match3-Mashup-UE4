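; Functional test checking that swapping two board pieces creates a match and scores it.
; It spawns a row of four connected piece holders, one holding a different type, and asserts that no pieces match initially.
; It then swaps the odd piece with its neighbor and, using timed delays, checks that only that piece survives and player 0 has the expected score before cleaning up.
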(event `self.ReceivePrepareTest`
  (for _index (range 4)
    (bind _returnvalue (`|SpawnActorFromClass` (select `bool` (== _index (`self.DifferentBoardPieceIndex`)) :`false` "/Game/Testing/ModifiedBPsForTest/Test_SpawnFastBoardPieceHolderType0BP.Test_SpawnFastBoardPieceHolderType0BP_C" :`true` "/Game/Testing/ModifiedBPsForTest/Test_SpawnFastBoardPieceHolderType1BP.Test_SpawnFastBoardPieceHolderType1BP_C" :!type "BoardPieceHolderCPP Class Reference") (`KismetMathLibrary.MakeTransform` (`KismetMathLibrary.MakeVector` 600.0 (* _index 500.0))) "Undefined" "OverrideRootScale" null null))
    (`KismetArrayLibrary.Array_Add` (`self.BoardPieceHolders`) _returnvalue))
  (`BoardPieceTestingUtilitiesCPP.SetConnectionsForBoardPieceHolders` (`self.BoardPieceHolders`) false self))

(event `self.ReceiveStartTest`
  (bind _differentboardpieceindex (`self.DifferentBoardPieceIndex`))
  (bind _boardpieceholders (`self.BoardPieceHolders`))
  (`KismetSystemLibrary.Delay` 0.1)
  (`self.GetBoardPiecesOfHoldersIntoArray`)
  (`KismetSystemLibrary.Delay` 0.75)
  (for _index (range (`KismetArrayLibrary.Array_Length` (`self.InitialBoardPieces`)))
    (`self.AssertEqual_Bool` (`KismetSystemLibrary.IsValid` (`|GetArrayItem` (`self.InitialBoardPieces`) _index)) true "No matches should occur here"))
  (`BoardPieceHolderCPP.DoSwap` (`|GetArrayItem` _boardpieceholders _differentboardpieceindex) (`|GetArrayItem` _boardpieceholders (+ _differentboardpieceindex 1)) 0)
  (`KismetSystemLibrary.Delay` 1.0)
  (for _index_2 (range (`KismetArrayLibrary.Array_Length` (`self.InitialBoardPieces`)))
    (`self.AssertEqual_Bool` (`KismetSystemLibrary.IsValid` (`|GetArrayItem` (`self.InitialBoardPieces`) _index_2)) (== _index_2 (`self.DifferentBoardPieceIndex`))))
  (`GameModeAndStateTestingUtilsCPP.IsPlayerIdInGameState` 0 self)
  (`GameModeAndStateTestingUtilsCPP.DoesPlayerHaveScore` 0 3 self)
  (`self.FinishTest` "Default")
  (`self.CleanupAfterTest`)
  (`GameModeAndStateTestingUtilsCPP.CleanUpAllGameplayThings` self))

(fn `UserConstructionScript`)