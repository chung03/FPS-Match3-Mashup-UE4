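; Functional test verifying that a spawned score pick-up falls to the ground and stays there.
; PrepareTest spawns a ScorePickUpBP in the air and stores a reference to it.
; StartTest waits, asserts the pick-up has dropped below a height threshold, records its location, then after another delay asserts it has not moved.
; It then finishes the test and destroys the pick-up.
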(event `self.ReceivePrepareTest`
  (bind _returnvalue (`|SpawnActorFromClass` "/Game/FirstPersonCPP/Blueprints/ScorePickups/ScorePickUpBP.ScorePickUpBP_C" (`KismetMathLibrary.MakeTransform` (300.0 0.0 300.0)) "Undefined" "OverrideRootScale" null null))
  (set `self.ScorePickUp` _returnvalue))

(event `self.ReceiveStartTest`
  (bind (_returnvalue_x _returnvalue_y _returnvalue_z) (`KismetMathLibrary.BreakVector` (`self.K2_GetActorLocation` (`self.ScorePickUp`))))
  (`KismetSystemLibrary.Delay` 1.5)
  (`self.AssertTrue` (< _returnvalue_z 150.0) "Score Pick Up should have dropped")
  (bind _output_get (set `self.ScorePickUpDroppedLocation` (`KismetMathLibrary.MakeVector` _returnvalue_x _returnvalue_y _returnvalue_z)))
  (`KismetSystemLibrary.Delay` 1.0)
  (`self.AssertEqual_Vector` (`self.K2_GetActorLocation` (`self.ScorePickUp`)) _output_get "Score Pick up should have stayed on the ground")
  (`self.FinishTest` "Default")
  (`self.K2_DestroyActor` (`self.ScorePickUp`)))

(fn `UserConstructionScript`)