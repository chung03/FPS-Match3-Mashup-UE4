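; Functional test verifying that a board piece holder replaces its board piece after lethal damage.
; PrepareTest spawns a fast-spawning test holder.
; StartTest deals massive server damage to the holder's current piece, then after a short delay asserts that a valid, different piece exists.
; It then finishes the test and destroys the holder.
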(event `self.ReceivePrepareTest`
  (bind _returnvalue (`|SpawnActorFromClass` "/Game/Testing/ModifiedBPsForTest/Test_SpawnFastBoardPieceHolderType0BP.Test_SpawnFastBoardPieceHolderType0BP_C" (`KismetMathLibrary.MakeTransform` (0.0 500.0 0.0)) "Undefined" "OverrideRootScale" null null))
  (set `self.BoardPieceHolder1` _returnvalue))

(event `self.ReceiveStartTest`
  (bind _currentboardpiece (`BoardPieceHolderCPP.CurrentBoardPiece` (`self.BoardPieceHolder1`)))
  (`KismetSystemLibrary.Delay` 1.0)
  (bind _output_get (set `self.BoardPiece1` (`BoardPieceHolderCPP.CurrentBoardPiece` (`self.BoardPieceHolder1`))))
  (`BoardPieceCPP.ServerDamagePiece` _output_get 0 999.0)
  (`KismetSystemLibrary.Delay` 1.0)
  (`self.AssertIsValid` _currentboardpiece "Board Piece Holder should create a new Board Piece after the current one is destroyed")
  (`self.AssertFalse` (== (`self.BoardPiece1`) _currentboardpiece) "After Board Piece is destroyed, a new Board Piece should be spawned")
  (`self.FinishTest` "Default")
  (`self.K2_DestroyActor` (`self.BoardPieceHolder1`)))

(fn `UserConstructionScript`)