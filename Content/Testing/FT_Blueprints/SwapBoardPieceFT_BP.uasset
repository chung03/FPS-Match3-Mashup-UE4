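; Functional test that verifies two board piece holders correctly swap their pieces.
; Preparation spawns two fast-spawning test holders and links them with a north-south connection.
; The test waits for pieces, calls DoSwap, waits again, then asserts each piece sits at the other holder's location with correct mutual ownership before finishing and cleaning up gameplay objects.
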(event `self.ReceivePrepareTest`
  (bind _returnvalue (`|SpawnActorFromClass` "/Game/Testing/ModifiedBPsForTest/Test_SpawnFastBoardPieceHolderType0BP.Test_SpawnFastBoardPieceHolderType0BP_C" (`KismetMathLibrary.MakeTransform` (0.0 500.0 0.0)) "Undefined" "OverrideRootScale" null null))
  (set `self.BoardPieceHolder1` _returnvalue)
  (bind _returnvalue_2 (`|SpawnActorFromClass` "/Game/Testing/ModifiedBPsForTest/Test_SpawnFastBoardPieceHolderType0BP.Test_SpawnFastBoardPieceHolderType0BP_C" (`KismetMathLibrary.MakeTransform` (0.0 -500.0 0.0)) "Undefined" "OverrideRootScale" null null))
  (set `self.BoardPieceHolder2` _returnvalue_2)
  (`BoardPieceTestingUtilitiesCPP.SetConnectionsForBoardPieceHolders` (`|MakeArray` (`self.BoardPieceHolder1`) (`self.BoardPieceHolder2`) :!type "BoardPieceHolderCPP Object Reference") true self))

(event `self.ReceiveStartTest`
  (`KismetSystemLibrary.Delay` 1.0)
  (set `self.BoardPiece1` (`BoardPieceHolderCPP.CurrentBoardPiece` (`self.BoardPieceHolder1`)))
  (set `self.BoardPiece2` (`BoardPieceHolderCPP.CurrentBoardPiece` (`self.BoardPieceHolder2`)))
  (`BoardPieceTestingUtilitiesCPP.IsBoardPieceAtHolder` (`self.BoardPieceHolder1`) self)
  (`BoardPieceTestingUtilitiesCPP.IsBoardPieceAtHolder` (`self.BoardPieceHolder2`) self)
  (`BoardPieceHolderCPP.DoSwap` (`self.BoardPieceHolder1`) (`self.BoardPieceHolder2`) 0)
  (`KismetSystemLibrary.Delay` 1.0)
  (`self.AssertEqual_Vector` (`self.K2_GetActorLocation` (`self.BoardPiece2`)) (`self.K2_GetActorLocation` (`self.BoardPieceHolder1`)))
  (`self.AssertEqual_Vector` (`self.K2_GetActorLocation` (`self.BoardPiece1`)) (`self.K2_GetActorLocation` (`self.BoardPieceHolder2`)))
  (`BoardPieceTestingUtilitiesCPP.IsBoardPieceOwnershipCorrect` (`self.BoardPieceHolder2`) (`self.BoardPiece1`) self)
  (`BoardPieceTestingUtilitiesCPP.IsBoardPieceOwnershipCorrect` (`self.BoardPieceHolder1`) (`self.BoardPiece2`) self)
  (`self.FinishTest` "Default")
  (`GameModeAndStateTestingUtilsCPP.CleanUpAllGameplayThings` self))

(fn `Board Piece Ownership Check`
  (params (BoardPiece :type "BoardPieceCPP Object Reference") (BoardPieceHolder :type "BoardPieceHolderCPP Object Reference") (BoardPieceHolderOwnershipFail :type String) (BoardPieceOwnershipFail :type String))
  (`self.AssertEqual_Bool` (== BoardPiece (`BoardPieceHolderCPP.CurrentBoardPiece` BoardPieceHolder)) true BoardPieceHolderOwnershipFail)
  (`self.AssertEqual_Bool` (== (`BoardPieceCPP.OwningPieceHolder` (`local.BoardPiece`)) (`local.BoardPieceHolder`)) true BoardPieceOwnershipFail))

(fn `UserConstructionScript`)