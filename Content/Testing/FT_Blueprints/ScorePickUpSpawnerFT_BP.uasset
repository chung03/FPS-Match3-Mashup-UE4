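; Functional test Blueprint that checks the score pickup spawner produces the expected number of pickups.
; PrepareTest spawns a Test_ScorePickUpSpawnerBP, and StartTest waits a fixed delay before asserting that five ScorePickUpBP actors exist in the world.
; It then finishes the test and destroys the spawner and every pickup found.
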(event `self.ReceivePrepareTest`
  (bind _returnvalue (`|SpawnActorFromClass` "/Game/Testing/ModifiedBPsForTest/Test_ScorePickUpSpawnerBP.Test_ScorePickUpSpawnerBP_C" (`KismetMathLibrary.MakeTransform` (0.0 500.0 0.0)) "Undefined" "OverrideRootScale" null null))
  (set `self.ScoreSpawner` _returnvalue))

(event `self.ReceiveStartTest`
  (`KismetSystemLibrary.Delay` 5.5)
  (bind _outactors (`GameplayStatics.GetAllActorsOfClass` "/Game/FirstPersonCPP/Blueprints/ScorePickups/ScorePickUpBP.ScorePickUpBP_C"))
  (bind _output_get (set `self.SpawnedScorePickUps` _outactors))
  (`self.AssertEqual_Int` (`KismetArrayLibrary.Array_Length` _output_get) 5 "There should be 5 score pickups spawned")
  (`self.FinishTest` "Default")
  (`self.K2_DestroyActor` (`self.ScoreSpawner`))
  (for _array_element (`self.SpawnedScorePickUps`)
    (`self.K2_DestroyActor` _array_element)))

(fn `UserConstructionScript`)