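; Functional test Blueprint that checks a board piece holder spawns its current board piece at the holder's own location.
; PrepareTest spawns a Test_SpawnFastBoardPieceHolderBP at a fixed offset and stores it.
; StartTest waits a second, asserts the piece's location equals the holder's, finishes the test and destroys the holder.
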(event `self.ReceivePrepareTest`
  (bind _returnvalue (`|SpawnActorFromClass` "/Game/Testing/ModifiedBPsForTest/Test_SpawnFastBoardPieceHolderBP.Test_SpawnFastBoardPieceHolderBP_C" (`KismetMathLibrary.MakeTransform` (0.0 500.0 0.0)) "Undefined" "OverrideRootScale" null null))
  (set `self.BoardPieceHolder` _returnvalue))

(event `self.ReceiveStartTest`
  (bind _boardpieceholder (`self.BoardPieceHolder`))
  (`KismetSystemLibrary.Delay` 1.0)
  (`self.AssertEqual_Vector` (`self.K2_GetActorLocation` (`BoardPieceHolderCPP.CurrentBoardPiece` _boardpieceholder)) (`self.K2_GetActorLocation` _boardpieceholder))
  (`self.FinishTest` "Default")
  (`self.K2_DestroyActor` (`self.BoardPieceHolder`)))

(fn `UserConstructionScript`)