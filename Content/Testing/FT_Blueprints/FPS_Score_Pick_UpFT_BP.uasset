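; Functional test Blueprint verifying that a score pickup is destroyed when it lands on the first-person character.
; PrepareTest spawns a ScorePickUpBP directly above a FirstPersonCharacter at the same horizontal position.
; StartTest waits briefly, asserts the pickup is no longer valid, finishes the test, then destroys the character and any surviving pickup.
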(event `self.ReceivePrepareTest`
  (bind _returnvalue (`|SpawnActorFromClass` "/Game/FirstPersonCPP/Blueprints/ScorePickups/ScorePickUpBP.ScorePickUpBP_C" (`KismetMathLibrary.MakeTransform` (0.0 500.0 200.0)) "Undefined" "OverrideRootScale" null null))
  (set `self.ScorePickUp` _returnvalue)
  (bind _returnvalue_2 (`|SpawnActorFromClass` "/Game/FirstPersonCPP/Blueprints/FirstPersonCharacter.FirstPersonCharacter_C" (`KismetMathLibrary.MakeTransform` (0.0 500.0 80.0)) "AlwaysSpawn" "OverrideRootScale" null null))
  (set `self.FPSChar1` _returnvalue_2))

(event `self.ReceiveStartTest`
  (bind _scorepickup (`self.ScorePickUp`))
  (`KismetSystemLibrary.Delay` 1.0)
  (`self.AssertFalse` (`KismetSystemLibrary.IsValid` (`self.ScorePickUp`)) "After Score Pick Up lands on top of the FPS character, the Score Pick Up should be destroyed")
  (`self.FinishTest` "Default")
  (`self.K2_DestroyActor` (`self.FPSChar1`))
  (`/Engine/EditorBlueprintResources/StandardMacros.IsValid` _scorepickup
    (:`Is Valid`
      (`self.K2_DestroyActor` _scorepickup))))

(fn `UserConstructionScript`)