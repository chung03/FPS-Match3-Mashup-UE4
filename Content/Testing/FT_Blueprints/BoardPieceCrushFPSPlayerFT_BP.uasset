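; Functional test verifying that a board piece spawning on top of an FPS character crushes and destroys it.
; PrepareTest spawns a fast board-piece holder test actor and a FirstPersonCharacter just above it, assigning the character's owning player ID.
; StartTest waits briefly, asserts the character is no longer valid, checks that player's expected score, then finishes and cleans up all gameplay actors.
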(event `self.ReceivePrepareTest`
  (bind _returnvalue (`|SpawnActorFromClass` "/Game/Testing/ModifiedBPsForTest/Test_SpawnFastBoardPieceHolderType0BP.Test_SpawnFastBoardPieceHolderType0BP_C" (`KismetMathLibrary.MakeTransform` (0.0 500.0 0.0)) "Undefined" "OverrideRootScale" null null))
  (set `self.BoardPieceHolder1` _returnvalue)
  (bind _returnvalue_2 (`|SpawnActorFromClass` "/Game/FirstPersonCPP/Blueprints/FirstPersonCharacter.FirstPersonCharacter_C" (`KismetMathLibrary.MakeTransform` (0.0 500.0 80.0)) "AlwaysSpawn" "OverrideRootScale" null null))
  (bind _output_get (set `self.FPSChar1` _returnvalue_2))
  (`F3MashUpCharacter.SetOwningPlayerID` _output_get (`self.PlayerId`)))

(event `self.ReceiveStartTest`
  (`KismetSystemLibrary.Delay` 1.0)
  (`self.AssertFalse` (`KismetSystemLibrary.IsValid` (`self.FPSChar1`)) "After Board Piece spawns on top of the FPS character, the FPS character should be destroyed")
  (`GameModeAndStateTestingUtilsCPP.DoesPlayerHaveScore` (`self.PlayerId`) (`self.ExpectedPlayerScore`) self)
  (`self.FinishTest` "Default")
  (`GameModeAndStateTestingUtilsCPP.CleanUpAllGameplayThings` self))

(fn `UserConstructionScript`)