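; Functional test that checks a first-person player can shoot a board piece, score a point and trigger a respawn.
; Setup spawns a fast-spawning test piece holder and a FirstPersonCharacter owned by player 0.
; After a delay it fires, then asserts the original piece is destroyed, the holder has a new one, and player 0 is in the game state with one point, before cleaning up gameplay objects.
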(event `self.ReceivePrepareTest`
  (bind _returnvalue (`|SpawnActorFromClass` "/Game/Testing/ModifiedBPsForTest/Test_SpawnFastBoardPieceHolderType0BP.Test_SpawnFastBoardPieceHolderType0BP_C" (`KismetMathLibrary.MakeTransform` (0.0 500.0 0.0)) "Undefined" "OverrideRootScale" null null))
  (set `self.BoardPieceHolder1` _returnvalue)
  (bind _returnvalue_2 (`|SpawnActorFromClass` "/Game/FirstPersonCPP/Blueprints/FirstPersonCharacter.FirstPersonCharacter_C" (`KismetMathLibrary.MakeTransform` (-400.0 500.0 80.0)) "AlwaysSpawn" "OverrideRootScale" null null))
  (bind _output_get (set `self.FPSChar1` _returnvalue_2))
  (`F3MashUpCharacter.SetOwningPlayerID` _output_get 0))

(event `self.ReceiveStartTest`
  (bind _currentboardpiece (`BoardPieceHolderCPP.CurrentBoardPiece` (`self.BoardPieceHolder1`)))
  (`KismetSystemLibrary.Delay` 1.0)
  (set `self.BoardPiece1` (`BoardPieceHolderCPP.CurrentBoardPiece` (`self.BoardPieceHolder1`)))
  (`F3MashUpCharacter.OnFire` (`self.FPSChar1`))
  (`KismetSystemLibrary.Delay` 1.0)
  (`self.AssertIsValid` _currentboardpiece "Board Piece Holder should create a new Board Piece after the current one is destroyed")
  (`self.AssertFalse` (== (`self.BoardPiece1`) _currentboardpiece) "After Board Piece is destroyed, a new Board Piece should be spawned")
  (`self.AssertFalse` (`KismetSystemLibrary.IsValid` (`self.BoardPiece1`)) "The first Board Piece should be destroyed")
  (`GameModeAndStateTestingUtilsCPP.IsPlayerIdInGameState` 0 self)
  (`GameModeAndStateTestingUtilsCPP.DoesPlayerHaveScore` 0 1 self)
  (`self.FinishTest` "Default")
  (`GameModeAndStateTestingUtilsCPP.CleanUpAllGameplayThings` self))

(fn `UserConstructionScript`)