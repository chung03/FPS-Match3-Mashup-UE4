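; Parent functional test Blueprint for board piece tests, providing shared helpers and teardown.
; GetBoardPiecesOfHoldersIntoArray appends each holder's CurrentBoardPiece to InitialBoardPieces.
; CleanupAfterTest destroys every actor in BoardPieceHolders, then clears both arrays.
; Its event graph and construction script are empty, so it defines no test logic of its own.
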(fn `CleanupAfterTest`
  (for _index (range (`KismetArrayLibrary.Array_Length` (`self.BoardPieceHolders`)))
    (`self.K2_DestroyActor` (`|GetArrayItem` (`self.BoardPieceHolders`) _index)))
  (`KismetArrayLibrary.Array_Clear` (`self.BoardPieceHolders`))
  (`KismetArrayLibrary.Array_Clear` (`self.InitialBoardPieces`)))

(fn `GetBoardPiecesOfHoldersIntoArray`
  (for _index (range (`KismetArrayLibrary.Array_Length` (`self.BoardPieceHolders`)))
    (`KismetArrayLibrary.Array_Add` (`self.InitialBoardPieces`) (`BoardPieceHolderCPP.CurrentBoardPiece` (`|GetArrayItem` (`self.BoardPieceHolders`) _index)))))

(fn `UserConstructionScript`)