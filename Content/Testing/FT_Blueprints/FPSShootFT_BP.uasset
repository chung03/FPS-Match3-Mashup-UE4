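; Functional test that checks that a first-person character's shot reduces another character's health by one.
; PrepareTest spawns two FirstPersonCharacters a short distance apart along X.
; StartTest fires from the first, asserts the second's health equals its max minus one, then finishes the test and destroys both actors.
; The assertion runs immediately after firing, with no delay.
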(event `self.ReceivePrepareTest`
  (bind _returnvalue (`|SpawnActorFromClass` "/Game/FirstPersonCPP/Blueprints/FirstPersonCharacter.FirstPersonCharacter_C" (`KismetMathLibrary.MakeTransform` (0.0 100.0 0.0)) "AlwaysSpawn" "OverrideRootScale" null null))
  (set `self.FPSChar_1` _returnvalue)
  (bind _returnvalue_2 (`|SpawnActorFromClass` "/Game/FirstPersonCPP/Blueprints/FirstPersonCharacter.FirstPersonCharacter_C" (`KismetMathLibrary.MakeTransform` (200.0 100.0 0.0)) "AlwaysSpawn" "OverrideRootScale" null null))
  (set `self.FPSChar_2` _returnvalue_2))

(event `self.ReceiveStartTest`
  (bind _fpschar_2 (`self.FPSChar_2`))
  (`F3MashUpCharacter.OnFire` (`self.FPSChar_1`))
  (bind _returnvalue (`F3MashUpCharacter.GetHealth` _fpschar_2))
  (bind _returnvalue_2 (`F3MashUpCharacter.GetMaxHealth` _fpschar_2))
  (`self.AssertEqual_Float` _returnvalue (- _returnvalue_2 1.0) "Health of FPSChar_2 was not reduced as expected")
  (`self.FinishTest` "Default")
  (`self.K2_DestroyActor` (`self.FPSChar_1`))
  (`self.K2_DestroyActor` (`self.FPSChar_2`)))

(fn `UserConstructionScript`)