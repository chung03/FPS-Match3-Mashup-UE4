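; Functional test checking that board pieces forming a match at spawn get destroyed.
; Preparation spawns three fast-spawning type 0 piece holders in a line along Y and links them as non-north-south neighbours.
; After a brief delay it records the holders' pieces, waits again, asserts that none of those initial pieces is still valid, then finishes and cleans up.
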(event `self.ReceivePrepareTest`
  (for _index (range 3)
    (bind _returnvalue (`|SpawnActorFromClass` "/Game/Testing/ModifiedBPsForTest/Test_SpawnFastBoardPieceHolderType0BP.Test_SpawnFastBoardPieceHolderType0BP_C" (`KismetMathLibrary.MakeTransform` (`KismetMathLibrary.MakeVector` 0.0 (* _index 500.0))) "Undefined" "OverrideRootScale" null null))
    (`KismetArrayLibrary.Array_Add` (`self.BoardPieceHolders`) _returnvalue))
  (`BoardPieceTestingUtilitiesCPP.SetConnectionsForBoardPieceHolders` (`self.BoardPieceHolders`) false self))

(event `self.ReceiveStartTest`
  (`KismetSystemLibrary.Delay` 0.1)
  (`self.GetBoardPiecesOfHoldersIntoArray`)
  (`KismetSystemLibrary.Delay` 0.75)
  (for _index (range (`KismetArrayLibrary.Array_Length` (`self.InitialBoardPieces`)))
    (`self.AssertEqual_Bool` (`KismetSystemLibrary.IsValid` (`|GetArrayItem` (`self.InitialBoardPieces`) _index))))
  (`self.FinishTest` "Default")
  (`self.CleanupAfterTest`))

(fn `UserConstructionScript`)