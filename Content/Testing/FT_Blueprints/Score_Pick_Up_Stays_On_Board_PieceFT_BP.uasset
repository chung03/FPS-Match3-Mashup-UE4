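; Functional test that checks a score pick-up drops onto a board piece and stays there.
; PrepareTest spawns the pick-up above a scaled-up test fast-moving board piece.
; StartTest waits, asserts the pick-up's height lies between the allowed limits and records its location.
; After a second delay it asserts the location is unchanged, then finishes and destroys both actors.
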(event `self.ReceivePrepareTest`
  (bind _returnvalue (`|SpawnActorFromClass` "/Game/FirstPersonCPP/Blueprints/ScorePickups/ScorePickUpBP.ScorePickUpBP_C" (`KismetMathLibrary.MakeTransform` (0.0 500.0 700.0)) "Undefined" "OverrideRootScale" null null))
  (set `self.ScorePickUp` _returnvalue)
  (bind _returnvalue_2 (`|SpawnActorFromClass` "/Game/Testing/ModifiedBPsForTest/Test_FastMoveBoardPieceType0BP.Test_FastMoveBoardPieceType0BP_C" (`KismetMathLibrary.MakeTransform` (0.0 500.0 0.0) (struct) (5.0 5.0 5.0)) "Undefined" "OverrideRootScale" null null))
  (set `self.BoardPiece` _returnvalue_2))

(event `self.ReceiveStartTest`
  (bind (_returnvalue_x _returnvalue_y _returnvalue_z) (`KismetMathLibrary.BreakVector` (`self.K2_GetActorLocation` (`self.ScorePickUp`))))
  (bind (_returnvalue_x_2 _returnvalue_y_2 _returnvalue_z_2) (`KismetMathLibrary.BreakVector` (`self.K2_GetActorLocation` (`self.ScorePickUp`))))
  (`KismetSystemLibrary.Delay` 1.5)
  (`self.AssertTrue` (< _returnvalue_z (`self.MaxAllowedScorePickUpHeight`)) "Score Pick Up should have dropped")
  (set `self.ScorePickUpDroppedLocation` (`KismetMathLibrary.MakeVector` _returnvalue_x _returnvalue_y _returnvalue_z))
  (`self.AssertTrue` (> _returnvalue_z_2 (`self.MinAllowedScorePickUpHeight`)) "Score Pick Up should not have touched the ground")
  (`KismetSystemLibrary.Delay` 1.0)
  (`self.AssertEqual_Vector` (`self.K2_GetActorLocation` (`self.ScorePickUp`)) (`self.ScorePickUpDroppedLocation`) "Score Pick up should have stayed on the Board Piece")
  (`self.FinishTest` "Default")
  (`self.K2_DestroyActor` (`self.ScorePickUp`))
  (`self.K2_DestroyActor` (`self.BoardPiece`)))

(fn `UserConstructionScript`)