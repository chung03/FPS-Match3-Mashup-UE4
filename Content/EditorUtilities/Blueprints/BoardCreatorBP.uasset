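; Editor utility that builds a rectangular game board of BoardPieceHolderBP actors.
; CreateBoardInEditor destroys previously tracked pieces, spawns one holder per cell, then positions and links them.
; Holders form an evenly spaced grid centered on BoardOrigin, stored in a flat array indexed row-major.
; Each holder's ConnectedBoardPieceHolders receives its in-bounds orthogonal neighbors at fixed direction slots, skipping off-board directions.
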(event `self.ReceiveBeginPlay`)

(fn `CreateBoardInEditor`
  (`self.RemoveExistingPieces`)
  (`self.InitializeBoardPieces`)
  (`self.MoveAndConnectPieces`))

(fn `GetArrayIndex`
  (params (Row :type Integer) (Column :type Integer))
  (returns (ArrayIndex :type Integer))
  (return (+ (* Row (`self.NumColumns`)) Column)))

(fn `InitializeBoardPieces`
  (for _ (range (* (`self.NumRows`) (`self.NumColumns`)))
    (bind _returnvalue (`|SpawnActorFromClass` "/Game/FirstPersonCPP/Blueprints/BoardPieces/BoardPieceHolderBP.BoardPieceHolderBP_C" (`KismetMathLibrary.MakeTransform` (`self.BoardOrigin`)) "Undefined" "OverrideRootScale" null null))
    (`KismetArrayLibrary.Array_Add` (`self.CurrentBoardPieces`) _returnvalue)))

(fn `MoveAndConnectPieces`
  (for _index (range (`self.NumRows`))
    (for _index_2 (range (`self.NumColumns`))
      (bind _arrayindex (`self.GetArrayIndex` _index _index_2))
      (`self.SetBoardPieceLocation` _arrayindex _index _index_2)
      (`self.SetBoardPieceConnections` _arrayindex _index _index_2))))

(fn `RemoveExistingPieces`
  (for _array_element (`self.CurrentBoardPieces`)
    (`self.K2_DestroyActor` _array_element))
  (`KismetArrayLibrary.Array_Clear` (`self.CurrentBoardPieces`)))

(fn `SetBoardPieceConnections`
  (params (ArrayIndex :type Integer) (Row :type Integer) (Column :type Integer))
  (bind _output (`|GetArrayItem` (`self.CurrentBoardPieces`) ArrayIndex))
  (`self.SetConnectionIfValid` 0 (+ Row 1) Column _output)
  (`self.SetConnectionIfValid` 1 (- Row 1) Column _output)
  (`self.SetConnectionIfValid` 2 Row (+ Column 1) _output)
  (`self.SetConnectionIfValid` 3 Row (- Column 1) _output))

(fn `SetBoardPieceLocation`
  (params (ArrayIndex :type Integer) (Row :type Integer) (Column :type Integer))
  (`self.K2_SetActorLocation` (`|GetArrayItem` (`self.CurrentBoardPieces`) ArrayIndex) (+ (`self.BoardOrigin`) (- (* (`KismetMathLibrary.MakeVector` (`KismetMathLibrary.Conv_IntToDouble` Row) (`KismetMathLibrary.Conv_IntToDouble` Column)) (`self.DistanceBetweenPieces`)) (/ (* (`KismetMathLibrary.MakeVector` (`KismetMathLibrary.Conv_IntToDouble` (- (`self.NumRows`) 1)) (`KismetMathLibrary.Conv_IntToDouble` (- (`self.NumColumns`) 1))) (`self.DistanceBetweenPieces`)) 2.0))) false false))

(fn `SetConnectionIfValid`
  (params (ConnectionIndex :type Integer) (OtherRow :type Integer) (OtherColumn :type Integer) (BoardPieceHolder :type "BoardPieceHolderCPP Object Reference"))
  (if (and (< OtherRow (`self.NumRows`)) (>= OtherRow 0) (< OtherColumn (`self.NumColumns`)) (>= OtherColumn 0))
    (bind _arrayindex (`self.GetArrayIndex` OtherRow OtherColumn))
    (`KismetArrayLibrary.Array_Set` (`BoardPieceHolderCPP.ConnectedBoardPieceHolders` BoardPieceHolder) ConnectionIndex (`|GetArrayItem` (`self.CurrentBoardPieces`) _arrayindex))))

(fn `UserConstructionScript`)